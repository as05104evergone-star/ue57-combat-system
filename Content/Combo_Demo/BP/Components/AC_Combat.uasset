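; AC_Combat is a character combat component handling weapon equipping and light-attack combos.
; On authority BeginPlay it async-loads a spear from DT_WeaponDetails onto the back socket; Left Alt montages move it between back and hand.
; Left click, gated by InputEnabled, plays the weapon's montages by combo index and caches camera-relative input direction.
; Tick eases yaw toward that direction and box-traces weapon sockets across frames, only printing hit Damage-tagged components.
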(event Custom|SpawnWeaponOnBack
  (params (DataRow :type Name))
  ;[0.15 0.15 0.15 0.5] 把武器生成到玩家背部
  (if (not (and (== DataRow (Variables|武器|GetEquippedWeaponRow)) (Utilities|IsValid (Variables|武器|GetCurrentWeapon)))) ; 不同时满足，则说明玩家没有装备武器，我们进行装备；满足了，则已经装备了，不进行重复装备
    (bind _output_get (Variables|武器|SetPendingWeaponRow DataRow))
    (bind _returnvalue (Utilities|GetDataTableRow "/Game/Combo_Demo/BP/DataTables/DT_WeaponDetails.DT_WeaponDetails" _output_get)
      (:then
        (bind _class (Utilities|AsyncLoadClassAsset (.EquipmentActor (Utilities|Struct|BreakBS_WeaponDetails _returnvalue)))
          (:Completed
            (if (Utilities|IsValid (Variables|武器|GetCurrentWeapon))
              (Actor|DestroyActor (Variables|武器|GetCurrentWeapon))
              (Variables|武器|SetCurrentWeapon 0)
              (Variables|武器|SetEquippedWeaponRow "None")
              (Utilities|Casting|CastToActorClass (stale _asactor))
              (else
                (bind _asactor (Utilities|Casting|CastToActorClass _class))
                (bind _returnvalue_2 (Game|SpawnActorfromClass _asactor (Transformation|GetActorTransform (Components|GetOwner)) "Undefined" "MultiplyWithRoot" 0 0))
                (bind _output_get_2 (Variables|武器|SetCurrentWeapon _returnvalue_2))
                (Transformation|AttachComponentToComponent _output_get_2 (Variables|/Script/Engine.Character|GetMesh (Variables|角色|GetOwningCharacter)) (.SocksNames_Back (Utilities|Struct|BreakBS_WeaponDetails _returnvalue)) "SnapToTarget" "SnapToTarget" "SnapToTarget" true) ; 注意这里的parent才是要被添加武器的项
                (Variables|武器|SetEquippedWeaponRow (Variables|武器|GetPendingWeaponRow))
                (Variables|状态判断|SetbWeaponBusy false)
                (Variables|状态判断|SetbWeaponInHand false)))))))))

(event Custom|UnequipWeapon
  (params (DataRaw :type Name))
  ;[0.15 0.15 0.15 0.5] 角色卸武器到背上
  (bind _returnvalue (Utilities|GetDataTableRow "/Game/Combo_Demo/BP/DataTables/DT_WeaponDetails.DT_WeaponDetails" DataRaw)
    (:then
      (Transformation|AttachComponentToComponent (Variables|武器|GetCurrentWeapon) (Variables|/Script/Engine.Character|GetMesh (Variables|角色|GetOwningCharacter)) (.SocksNames_Back (Utilities|Struct|BreakBS_WeaponDetails _returnvalue)) "SnapToTarget" "SnapToTarget" "SnapToTarget" true) ; 注意这里的parent才是要被添加武器的项
      (Variables|状态判断|SetbWeaponInHand false)
      (Variables|武器|SetEquippedWeaponRow "None"))))

(event Custom|EquipWeapon
  (params (DataRow :type Name))
  ;[0.15 0.15 0.15 0.5] 角色装武器到手上
  (if (not (Variables|状态判断|GetbWeaponInHand))
    (bind _output_get (Variables|武器|SetPendingWeaponRow DataRow))
    (bind _returnvalue (Utilities|GetDataTableRow "/Game/Combo_Demo/BP/DataTables/DT_WeaponDetails.DT_WeaponDetails" _output_get)
      (:then
        (Transformation|AttachComponentToComponent (Variables|武器|GetCurrentWeapon) (Variables|/Script/Engine.Character|GetMesh (Variables|角色|GetOwningCharacter)) (.SocksNames_Hand (Utilities|Struct|BreakBS_WeaponDetails _returnvalue)) "SnapToTarget" "SnapToTarget" "SnapToTarget" true) ; 注意这里的parent才是要被添加武器的项
        (Variables|状态判断|SetbWeaponInHand true)
        (Variables|武器|SetEquippedWeaponRow (Variables|Default|GetData%20Row))
        (Variables|武器|SetPendingWeaponRow "None")))))

(event EventBeginPlay
  ;[0.15 0.009642 0.001389 0.5] 从角色基类获取到当前拥有该组件的角色，把该初始化的东西都初始化
  (Networking|SwitchHasAuthority
    (:Authority
      (bind _as角色 (Utilities|Casting|CastToCharacter (Components|GetOwner))) ; 从角色基类去获取到带该组件的角色
      (Variables|角色|SetOwningCharacter _as角色)
      (CallFunction|SpawnWeapononBack "Spear"))))

(event EventCallWeaponTrace
  (params (WeaponTraceOn :type Boolean))
  ;[0.15 0.15 0.15 0.5] 命中检测接口
  (Variables|状态判断|SetWeapon%20Trace%20On WeaponTraceOn)
  (bind _weaponmesh (Class|BPIWeaponActor|GetWeaponMesh(Message) (Variables|武器|GetCurrentWeapon)))
  (Variables|Default|SetPreviousTopTrace (Transformation|GetSocketLocation _weaponmesh "Top"))
  (Variables|Default|SetPreviousBottomTrace (Transformation|GetSocketLocation _weaponmesh "Bottom")))

(event EventTick
  (params (DeltaSeconds :type Float%20%28single-precision%29))
  (bind _owningcharacter (Variables|角色|GetOwningCharacter))
  (bind _returnvalue (Transformation|GetActorRotation _owningcharacter))
  ;[0.15 0.15 0.15 0.5] 根据玩家朝向更改攻击方向的逻辑实现；武器实时命中检测
  (Transformation|SetActorRotation (Variables|角色|GetOwningCharacter) (Math|Rotator|MakeRotator (.roll _returnvalue) (.pitch _returnvalue) (.yaw (Math|Interpolation|RInterpTo (Transformation|GetActorRotation (Variables|角色|GetOwningCharacter)) (Variables|角色|GetCachedInputRotation) DeltaSeconds 13.0))))
  (CallFunction|PlayWeaponTrace))

(event EventCallSetMovementVector
  (params (MovementVectors :type BS%20Movement%20Vector%20Structure))
  ;[0.15 0.15 0.15 0.5] 获取玩家当前的移动方向向量（这里只是接口，具体逻辑接在了角色的移动输入后面）
  (Variables|角色|SetCurrentMovementVector MovementVectors))

(event EventCallSetInputEnabled
  (params (Enabled :type Boolean))
  ;[0.15 0.15 0.15 0.5] 讲玩家状态设置为可以进行输入
  (bind _output_get (Variables|状态判断|SetInputEnabled Enabled))
  (if _output_get
    (Components|Tick|SetComponentTickEnabled true)))

(event Input|KeyboardEvents|LeftAlt
  (params (Key :type Key%20Structure :default "None"))
  (bind _owningcharacter (Variables|角色|GetOwningCharacter))
  (bind _data_row (Variables|Default|GetData%20Row))
  (bind _mesh (Variables|/Script/Engine.Character|GetMesh _owningcharacter))
  ;[0.15 0.15 0.15 0.5] 装上/卸下装备按键逻辑
  (:Pressed
    (if (== (Variables|状态判断|GetbWeaponBusy) false) ; 防连按机制
      (if (Variables|状态判断|GetbWeaponInHand) ; 有武器放卸下，没武器放装上
        (Variables|状态判断|SetbWeaponBusy true)
        (Animation|Montage|PlayMontage _mesh "/Game/Combo_Demo/Animation/Montage/AM_Unequip.AM_Unequip"
          (:OnCompleted
            (CallFunction|UnequipWeapon _data_row :!label _label))
          (:OnInterrupted
            _)
          (:OnNotifyBegin
            (goto _label)))
        (Variables|状态判断|SetbWeaponBusy false)
        (else
          (Variables|状态判断|SetbWeaponBusy true)
          (Animation|Montage|PlayMontage _mesh "/Game/Combo_Demo/Animation/Montage/AM_Equip.AM_Equip"
            (:OnCompleted
              (CallFunction|EquipWeapon _data_row :!label _label_2))
            (:OnInterrupted
              _)
            (:OnNotifyBegin
              (goto _label_2)))
          (Variables|状态判断|SetbWeaponBusy false))))))

(event Input|MouseEvents|LeftMouseButton
  (params (Key :type Key%20Structure))
  ;[0.15 0.15 0.15 0.5] 按左键进行普攻连招
  (:Pressed
    (bind _inputenabled (CallFunction|CheckBufferedInput "NewEnumerator0"))
    (if _inputenabled
      (CallFunction|LightAttack)
      (Utilities|FlowControl|RetriggerableDelay 2.0) ; 打完一套设置延迟，防止无限连
      (Variables|连招|SetComboIndex 0)
      (Variables|连招|SetCurrentBufferedInput "NewEnumerator0"))))

(fn GetCharacterMovementDirection
  (bind _returnvalue (Game|GetPlayerController 0))
  (bind _returnvalue_2 (Pawn|GetControlRotation _returnvalue :!class /Script/Engine.Controller))
  (bind _returnvalue_3 (Math|Rotator|MakeRotator 0.0 0.0 (.yaw _returnvalue_2)))
  (return (Math|Vector|GetForwardVector _returnvalue_3) (Math|Vector|GetRightVector _returnvalue_3)))

(fn GetInputRotation
  (bind (_forwardvector _rightvector) (CallFunction|GetCharacterMovementDirection))
  (bind _owningcharacter (Variables|角色|GetOwningCharacter))
  (bind _currentmovementvector (Variables|角色|GetCurrentMovementVector))
  (bind _returnvalue (Transformation|GetActorLocation _owningcharacter))
  (return (Math|Rotator|FindLookatRotation _returnvalue (+ _returnvalue (* _forwardvector (.y _currentmovementvector)) (* _rightvector (.x _currentmovementvector))))))

(fn LightAttack
  (if (Variables|状态判断|GetbWeaponInHand)
    (bind _attackmontages (Class|BPIWeaponActor|GetAttackMontages(Message) (Variables|武器|GetCurrentWeapon)))
    (Animation|PlayAnimMontage (Variables|角色|GetOwningCharacter) (Utilities|Array|Get(acopy) _attackmontages (Variables|连招|GetComboIndex)) 1.0 "None") ; 使用这个蒙太奇节点，函数也可以调用
    (bind _inputrotation (CallFunction|GetInputRotation)) ; 输入的旋转只影响z轴
    (Variables|角色|SetCachedInputRotation _inputrotation)
    (Components|Tick|SetComponentTickEnabled true)
    (bind _currentweapon (Variables|武器|GetCurrentWeapon) ; 角色有武器才允许播放
      (:then
        (bind _attackmontages_2 (Class|BPIWeaponActor|GetAttackMontages(Message) _currentweapon))
        (bind _result (Math|Integer|IncrementInt (Variables|连招|GetComboIndex)) ; 累加进行连招
          (:%20%20
            (Development|PrintText (Utilities|Text|ToText(Integer) _result))
            (Utilities|FlowControl|Sequence
              (:then_0
                (if (>= (Variables|连招|GetComboIndex) (Utilities|Array|Length _attackmontages_2))
                  (Variables|连招|SetComboIndex 0)))))))
      (:else))))

(fn CheckBufferedInput
  (params (AttackOrNot :type E_InputBuffered%20Enum :default "NewEnumerator0"))
  (if (Variables|状态判断|GetInputEnabled)
    (return true)
    (else
      (Variables|连招|SetCurrentBufferedInput AttackOrNot)
      (return false))))

(fn PlayWeaponTrace
  (if (Variables|状态判断|GetWeapon%20Trace%20On)
    (bind _currentweapon (Variables|武器|GetCurrentWeapon)
      (:then
        (bind _weaponmesh (Class|BPIWeaponActor|GetWeaponMesh(Message) _currentweapon))
        (LocalVariables|SetCurrentTopTrace (Transformation|GetSocketLocation _weaponmesh "Top"))
        (LocalVariables|SetCurrentBottomTrace (Transformation|GetSocketLocation _weaponmesh "Bottom"))
        (bind (_outhit _returnvalue) (Collision|BoxTraceByChannel (Variables|Default|GetPreviousTopTrace) (LocalVariables|GetCurrentTopTrace) (Math|Vector|MakeVector (/ (Math|Vector|Distance(Vector) (Variables|Default|GetPreviousTopTrace) (LocalVariables|GetCurrentBottomTrace)) 2.0) 0.0 0.0) (Math|Rotator|FindLookatRotation (Variables|Default|GetPreviousTopTrace) (LocalVariables|GetCurrentBottomTrace)) "TraceTypeQuery1" false 0 "ForDuration")) ; 从武器顶部到底部插槽建立碰撞箱，从上一帧起始，下一帧结束，保证缝隙不会过大；
        (Variables|Default|SetPreviousTopTrace (LocalVariables|GetCurrentTopTrace))
        (Variables|Default|SetPreviousBottomTrace (LocalVariables|GetCurrentBottomTrace))
        (if _returnvalue
          (Development|PrintString (Utilities|GetDisplayName (Class|Actor|FindComponentbyTag (.HitActor (Collision|BreakHitResult _outhit)) "/Script/Engine.ActorComponent" "Damage")))))
      (:else))))