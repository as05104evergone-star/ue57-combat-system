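; Enemy component running test melee attack logic against the player.
; A looping timer checks state and range, turns the owner by yaw toward the player, reads damage from DT_Enemy and plays the attack montage.
; DoAttackHit sphere-traces forward, dedupes targets per swing and applies GE_Damage unless ResolveDefense on the player returns dodged or parried.
; Parry stun blocks attacks and hits; StopAttack marks death, clearing the timer and stopping the montage.
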(event Custom|AttackLoop
  ;[0.15 0.15 0.15 0.5] 敌人攻击逻辑（测试版本）
  (Variables|角色|SetPlayer (Game|GetPlayerCharacter 0))
  (Utilities|IsValid (Variables|角色|GetOwningNPC)
    (:Is%20Valid
      (if (not (or (Variables|状态判断|GetbAttacking) (Variables|状态判断|GetbIsParryStunned))) ; 如果正在攻击或者被招架了或者敌人死亡了，不执行下一次攻击
        (if (not (Variables|状态判断|GetbDead))
          (if (not (> (Math|Vector|Distance(Vector) (Transformation|GetActorLocation (Variables|角色|GetOwningNPC)) (Transformation|GetActorLocation (Variables|角色|GetPlayer))) (Variables|数值|GetAttackRange))) ; 再攻击范围内，再执行攻击
            (if (not (Variables|/Game/Combo_Demo/BP/Components/AC_Combat.AC_Combat_C|GetbIsDead (Actor|GetComponentbyClass (Variables|角色|GetPlayer) "/Game/Combo_Demo/BP/Components/AC_Combat.AC_Combat_C")))
              (Transformation|SetActorRotation (Variables|角色|GetOwningNPC) (Math|Rotator|MakeRotator 0.0 0.0 (.yaw (Math|Rotator|FindLookatRotation (Transformation|GetActorLocation (Variables|角色|GetOwningNPC)) (Transformation|GetActorLocation (Variables|角色|GetPlayer)))))) ; 设置敌人攻击方向
              (bind _value (CallFunction|GetEnemyParam "/Game/Combo_Demo/BP/DataTables/DT_Enemy.DT_Enemy" "enemy.shadow.atk"))
              (Variables|数值|SetCurrentAttackDamage _value)
              (Utilities|Array|Clear (Variables|角色|GetHitTargetsThisSwing)) ; 命中判定去重
              (Variables|状态判断|SetbAttacking true)
              (Animation|Montage|PlayMontage (Variables|/Script/Engine.Character|GetMesh (Variables|角色|GetOwningNPC)) (Variables|角色|GetAttackMontage)
                (:OnCompleted
                  (Variables|状态判断|SetbAttacking false))
                (:OnInterrupted
                  (Variables|状态判断|SetbAttacking false))))))))))

(event EventBeginPlay
  (bind _as角色 (Utilities|Casting|CastToCharacter (Components|GetOwner)))
  (Variables|角色|SetOwningNPC _as角色)
  (bind _returnvalue (Utilities|Time|SetTimerbyEvent (delegate Custom|AttackLoop) (Variables|数值|GetAttackInterval) true))
  (Variables|数值|SetAttackLoopTimer _returnvalue))

(event EventTick
  (params (DeltaSeconds :type Float%20%28single-precision%29)))

(fn DoAttackHit
  (bind _owningnpc (Variables|角色|GetOwningNPC))
  (bind _owningnpc_2 (Variables|角色|GetOwningNPC))
  (Utilities|IsValid (Actor|GetComponentbyClass (Variables|角色|GetPlayer) "/Game/Combo_Demo/BP/Components/AC_Combat.AC_Combat_C")
    (:Is%20Valid
      (if (not (or (Variables|状态判断|GetbDead) (or (or (not (Variables|状态判断|GetbAttacking)) (Variables|状态判断|GetbIsParryStunned)) (Variables|/Game/Combo_Demo/BP/Components/AC_Combat.AC_Combat_C|GetbIsDead (Actor|GetComponentbyClass (Variables|角色|GetPlayer) "/Game/Combo_Demo/BP/Components/AC_Combat.AC_Combat_C"))))) ; 不在攻击/攻击被招架/玩家死了/自己死了，不执行下一步判定
        (Development|PrintString "执行攻击函数")
        (bind (_outhit _returnvalue) (Class|KismetSystemLibrary|SphereTraceSinglebyProfile (+ (Transformation|GetActorLocation _owningnpc_2) (* (Transformation|GetActorForwardVector _owningnpc_2) 5e+01)) (+ (Transformation|GetActorLocation _owningnpc) (* (Transformation|GetActorForwardVector _owningnpc) 1.6e+02)) 6e+01 "Pawn" false 0 "ForDuration" true))
        (if _returnvalue
          (Utilities|IsValid (.HitActor (Collision|BreakHitResult _outhit)) ; 防止未命中导致空对象报错
            (:Is%20Valid
              (if (not (Variables|/Game/Combo_Demo/BP/Components/AC_Combat.AC_Combat_C|GetbIsDead (Actor|GetComponentbyClass (.HitActor (Collision|BreakHitResult _outhit)) "/Game/Combo_Demo/BP/Components/AC_Combat.AC_Combat_C")))
                (if (not (Utilities|Array|ContainsItem (Variables|角色|GetHitTargetsThisSwing) (.HitActor (Collision|BreakHitResult _outhit))))
                  (Utilities|Array|Add (Variables|角色|GetHitTargetsThisSwing) (.HitActor (Collision|BreakHitResult _outhit)))
                  (bind _defenseresult (CallFunction|ResolveDefense (Variables|角色|GetPlayer) (Variables|角色|GetOwningNPC) (Variables|状态判断|GetbNextAttackParryable)))
                  (switch Utilities|FlowControl|Switch|SwitchonE_DefenseResult _defenseresult
                    (:NewEnumerator0
                      (Class|GASCombatStatics|ApplyDamagetoTarget (Variables|角色|GetOwningNPC) (.HitActor (Collision|BreakHitResult _outhit)) "/Game/Combo_Demo/BP/GAS/GE_Damage.GE_Damage_C" (Variables|数值|GetCurrentAttackDamage) 1 0))
                    (:NewEnumerator1
                      (Development|PrintString "BeDodged"))
                    (:NewEnumerator2
                      (Development|PrintString "BeParried"))))))))))))

(fn StopAttack
  (Variables|状态判断|SetbDead true)
  (Utilities|Time|ClearandInvalidateTimerbyHandle (Variables|数值|GetAttackLoopTimer))
  (Variables|状态判断|SetbAttacking false)
  (Variables|状态判断|SetbIsParryStunned false)
  (Utilities|Array|Clear (Variables|角色|GetHitTargetsThisSwing))
  (Animation|StopAnimMontage (Variables|角色|GetOwningNPC) (Variables|角色|GetAttackMontage)))